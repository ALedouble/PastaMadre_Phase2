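; BP_Joe is an enemy AI pawn that reacts to spotting the player, chases them and winds up for an attack.
; An enum state machine, switched through ChangeState, runs Surprised, Chase, Anticipation and Attack, though Attack has no behaviour here.
; Tick counts down randomised surprise and anticipation timers, smoothly turns toward the player and issues AIMoveTo until within shooting distance.
; Entering Surprised plays a timeline-driven mesh squash-and-stretch.
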(event Custom|PlayerSpotted
  ;[1 1 1] SURPRISE STATE
  (CallFunction|ChangeState "NewEnumerator1"))

(event Custom|ScaleWhenSurprised
  ;[1 1 1] SURPRISE STATE
  (Components|Timeline|SetPlayRate (Variables|Default|GetScaleTimeline) 3.0)
  (bind _lerpvalue (Timeline|ScaleTimeline PlayFromStart)
    (:Update
      (Transformation|SetRelativeScale3D (Variables|Character|GetMesh) (Math|Vector|Lerp(Vector) "1.000000,1.000000,1.000000" "0.800000,0.800000,1.200000" _lerpvalue)))))

(event Custom|DecreaseSurpriseTime
  ;[1 1 1] SURPRISE STATE
  (if (Utilities|Enum|Equal(Enum) (Variables|Default|GetMyState) "NewEnumerator1")
    (if (> (Variables|Surprise|GetSurpriseTime) 0.0)
      (Variables|Surprise|SetSurpriseTime (Math|Float|Clamp(Float) (- (Variables|Surprise|GetSurpriseTime) (Utilities|Time|GetWorldDeltaSeconds))))
      (else
        (CallFunction|ChangeState "NewEnumerator2")))))

(event Custom|RotateTowardsPlayer
  ;[1 1 1] ROTATION
  (switch Utilities|FlowControl|Switch|SwitchonENUM_AIState (Variables|Default|GetMyState)
    (:NewEnumerator1
      _)
    (:NewEnumerator2
      _)
    (:NewEnumerator3
      _))
  (Transformation|SetActorRotation (Math|Rotator|Lerp(Rotator) (Transformation|GetActorRotation) (Math|Rotator|FindLookatRotation (Transformation|GetActorLocation) (Transformation|GetActorLocation (Game|GetPlayerCharacter 0))) 0.1 true)))

(event Custom|Chase%20Player
  ;[1 1 1] CHASE STATE
  (if (Utilities|Enum|Equal(Enum) (Variables|Default|GetMyState) "NewEnumerator2")
    (AI|AIMoveTo self "0, 0, 0" (Game|GetPlayerCharacter 0) (Variables|Chase|GetMinDistanceToShoot) false
      (:OnSuccess
        (CallFunction|ChangeState "NewEnumerator3")))))

(event Custom|DecreaseAnticipationTime
  ;[1 1 1] ANTICIPATION STATE
  (if (Utilities|Enum|Equal(Enum) (Variables|Default|GetMyState) "NewEnumerator3")
    (if (> (Variables|Prepare|GetAnticipationTime) 0.0)
      (Variables|Prepare|SetAnticipationTime (Math|Float|Clamp(Float) (- (Variables|Prepare|GetAnticipationTime) (Utilities|Time|GetWorldDeltaSeconds)) 0.0))
      (else
        (CallFunction|ChangeState "NewEnumerator4")))))

(event EventTick
  (params (DeltaSeconds :type Float%20%28single-precision%29))
  (CallFunction|DecreaseSurpriseTime)
  (CallFunction|RotateTowardsPlayer)
  (CallFunction|ChasePlayer)
  (CallFunction|DecreaseAnticipationTime))

(fn ConstructionScript)

(fn EnterState
  (params (NewState :type ENUM_AIState%20Enum :default "NewEnumerator0"))
  (bind _randomisationsurprisetime (Variables|Surprise|GetRandomisationSurpriseTime))
  (bind _randomisationanticipationtime (Variables|Prepare|GetRandomisationAnticipationTime))
  (bind _output_get (Variables|Default|SetMyState NewState))
  (switch Utilities|FlowControl|Switch|SwitchonENUM_AIState _output_get
    (:NewEnumerator1
      (Variables|Surprise|SetSurpriseTime (+ (Math|Random|RandomFloatinRange (* _randomisationsurprisetime -1.0) _randomisationsurprisetime) (Variables|Surprise|GetMaxSurpriseTime)))
      (CallFunction|ScalewhenSurprised))
    (:NewEnumerator3
      (Variables|Prepare|SetAnticipationTime (+ (Math|Random|RandomFloatinRange (* _randomisationanticipationtime -1.0) _randomisationanticipationtime) (Variables|Prepare|GetMaxAnticipationTime))))))

(fn ExitState
  (switch Utilities|FlowControl|Switch|SwitchonENUM_AIState (Variables|Default|GetMyState)))

(fn ChangeState
  (params (NewState :type ENUM_AIState%20Enum :default "NewEnumerator0"))
  (Development|PrintString (Utilities|String|EnumtoString NewState))
  (CallFunction|ExitState)
  (CallFunction|EnterState NewState))