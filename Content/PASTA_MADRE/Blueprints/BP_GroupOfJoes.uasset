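; BP_GroupOfJoes is a group manager that shares player detection among a set of Joes.
; On BeginPlay it registers itself as MyGroup on every Joe in JoesInTheGroup.
; GroupSpottedPlayer changes the state of each Joe that has not yet detected the player, except the ExceptionIfHit Joe, which is only flagged as having detected the player.
; It then sets PlayerSpottedForEveryone.
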(event Custom|GroupSpottedPlayer
  (params (ExceptionIfHit :type BP%20Joe%20Object%20Reference))
  (for _array_element (Variables|Default|GetJoesInTheGroup)
    (if (not (Variables|/Game/PASTA_MADRE/Blueprints/BP_Joe.BP_Joe_C|GetPlayerDetected _array_element))
      (if (== _array_element ExceptionIfHit)
        (Variables|/Game/PASTA_MADRE/Blueprints/BP_Joe.BP_Joe_C|SetPlayerDetected _array_element true)
        (else
          (Default|ChangeState _array_element "NewEnumerator1")))))
  (Variables|Default|SetPlayerSpottedForEveryone true))

(event EventBeginPlay
  (for _array_element (Variables|Default|GetJoesInTheGroup)
    (Variables|/Game/PASTA_MADRE/Blueprints/BP_Joe.BP_Joe_C|SetMyGroup _array_element self)))

(fn ConstructionScript)