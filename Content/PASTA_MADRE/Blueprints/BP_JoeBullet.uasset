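; BP_JoeBullet is a projectile that damages the player character on overlap and then destroys itself.
; Each Tick it moves along BulletDirection at BulletSpeed, scaled by delta time, using an unswept world offset instead of a movement component.
; It ignores overlaps with any other actor and destroys itself when its Lifetime countdown drops below zero.
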(event Collision|EventActorBeginOverlap
  (params (OtherActor :type Actor%20Object%20Reference))
  (bind _returnvalue (Game|GetPlayerCharacter 0))
  (if (== OtherActor _returnvalue)
    (Game|Damage|ApplyDamage _returnvalue (Variables|Default|GetBulletDamage) 0 0)
    (Actor|DestroyActor)))

(event EventTick
  (params (DeltaSeconds :type Float%20%28single-precision%29))
  ;[1 1 1] TICK
  (Transformation|AddActorWorldOffset (* (Variables|Default|GetBulletDirection) (* (Variables|Default|GetBulletSpeed) (Utilities|Time|GetWorldDeltaSeconds))))
  (bind _output_get (Variables|Default|SetLifetime (- (Variables|Default|GetLifetime) (Utilities|Time|GetWorldDeltaSeconds))))
  (if (< _output_get 0.0)
    (Actor|DestroyActor)))

(fn ConstructionScript)